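; Camera pawn with a visible cursor that moves along its local axes and zooms by changing spring arm length within limits.
; Holding the middle mouse button hides the cursor and opens two gates that let mouse input rotate the view.
; Mouse X yaws the scene root, turning the movement axes with it, while mouse Y pitches an invisible anchor sphere within a clamped downward range.
; H prints actor rotation.
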(event `self.ReceiveBeginPlay`
  (set `PlayerController.bShowMouseCursor` true (`GameplayStatics.GetPlayerController` 0)))

(event `InputAxis|ZoomAxis`
  (params (AxisValue :type "Float (single-precision)"))
  (bind _springarm (`self.SpringArm`))
  (set `SpringArmComponent.TargetArmLength` (`KismetMathLibrary.FClamp` (+ (* AxisValue (`self.zoom_speed`) -1.0) (`SpringArmComponent.TargetArmLength` _springarm)) (`self.min_zoom`) (`self.max_zoom`)) _springarm))

(event `InputAxis|ForwardReverseAxis`
  (params (AxisValue :type "Float (single-precision)"))
  (`self.K2_AddActorLocalOffset` (`KismetMathLibrary.MakeVector` (* AxisValue (`self.move_speed`)))))

(event `InputAxis|LeftRightAxis`
  (params (AxisValue :type "Float (single-precision)"))
  (`self.K2_AddActorLocalOffset` (`KismetMathLibrary.MakeVector` 0.0 (* (`self.move_speed`) AxisValue))))

(event `InputAxisKey|MouseX`
  (params (AxisValue :type "Float (single-precision)"))
  (`/Engine/EditorBlueprintResources/StandardMacros.Gate` true :!label _label
    (:`Exit`
      (`SceneComponent.K2_AddLocalRotation` (`self.DefaultSceneRoot`) (`KismetMathLibrary.MakeRotator` 0.0 0.0 (* (`self.rotation_speed`) AxisValue)) false false))))

(event `Key|MiddleMouseButton`
  (params (Key :type "Key Structure" :default "AnyKey"))
  (bind _returnvalue (`GameplayStatics.GetPlayerController` 0))
  (bind _invisible_anchor_sphere (`self.invisible_anchor_sphere`))
  (bind (_returnvalue_roll _returnvalue_pitch _returnvalue_yaw) (`KismetMathLibrary.BreakRotator` (`SceneComponent.K2_GetComponentRotation` _invisible_anchor_sphere)))
  (:`Pressed`
    (set `PlayerController.bShowMouseCursor` false _returnvalue)
    (`|ExecutionSequence`
      (:`then_0`
        (goto _label :!via `Open`))
      (:`then_1`
        (goto _label_2 :!via `Open`))))
  (:`Released`
    (set `PlayerController.bShowMouseCursor` true _returnvalue)
    (`|ExecutionSequence`
      (:`then_0`
        (goto _label :!via `Close`))
      (:`then_1`
        (goto _label_2 :!via `Close`)))))

(event `InputAxisKey|MouseY`
  (params (AxisValue :type "Float (single-precision)"))
  (bind _invisible_anchor_sphere (`self.invisible_anchor_sphere`))
  (bind (_returnvalue_roll _returnvalue_pitch _returnvalue_yaw) (`KismetMathLibrary.BreakRotator` (`SceneComponent.K2_GetComponentRotation` _invisible_anchor_sphere)))
  (`/Engine/EditorBlueprintResources/StandardMacros.Gate` true :!label _label_2
    (:`Exit`
      (`SceneComponent.K2_SetWorldRotation` _invisible_anchor_sphere (`KismetMathLibrary.MakeRotator` _returnvalue_roll (`KismetMathLibrary.FClamp` (+ (* AxisValue (`self.rotation_speed`)) _returnvalue_pitch) -75.0 -15.0) _returnvalue_yaw) false false))))

(event `Key|H`
  (params (Key :type "Key Structure" :default "AnyKey"))
  (:`Pressed`
    (`KismetSystemLibrary.PrintString` (`KismetStringLibrary.Conv_RotatorToString` (`self.K2_GetActorRotation`)))))

(fn `UserConstructionScript`)